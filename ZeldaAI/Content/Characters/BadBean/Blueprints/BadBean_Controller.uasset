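; AI controller for the BadBean character that starts its behavior tree and seeds the blackboard with a patrol point and countdown.
; Perception updates record the seen actor and last seen position; losing sight clears only the seen actor, while forgetting clears the pawn's target.
; Patrol, target, attack and state calls pass through to the pawn as messages.
; Combat behavior is swappable through dynamic subtree injection.
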(event `self.ReceiveBeginPlay`
  (bind _blackboardcomponent (`self.UseBlackboard` "/Game/Characters/BadBean/Blueprints/BadBean_BB.BadBean_BB"))
  (bind _patrol_point (`self.Get_Patrol_Point` 0))
  (`BlackboardComponent.SetValueAsObject` _blackboardcomponent "Patrol_Point" _patrol_point)
  (`BlackboardComponent.SetValueAsFloat` _blackboardcomponent "CountdownTimer" 2.0)
  (`self.RunBehaviorTree` "/Game/Characters/BadBean/Blueprints/AI/BadBean_BT.BadBean_BT"))

(event `self.AIPerception.OnTargetPerceptionUpdated`
  (params (Actor :type "Actor Object Reference") (Stimulus :type "AIStimulus Structure"))
  (bind _returnvalue (`AIBlueprintHelperLibrary.GetBlackboard` null))
  (if Stimulus_bSuccessfullySensed
    (`BlackboardComponent.SetValueAsObject` _returnvalue "Seen_Player" Actor)
    (`BlackboardComponent.SetValueAsVector` _returnvalue "LastSeenPosition" Stimulus_StimulusLocation)
    (message `/Game/Combat_Interface.Set_Target` (`self.K2_GetPawn`) Actor)
    (else
      (`BlackboardComponent.ClearValue` _returnvalue "Seen_Player"))))

(event `self.AIPerception.OnTargetPerceptionForgotten`
  (params (Actor :type "Actor Object Reference"))
  (`KismetSystemLibrary.PrintString` "Forgot Target")
  (message `/Game/Combat_Interface.Set_Target` (`self.K2_GetPawn`) null))

(event `self.Update_State`
  (params (New_State :type "/Game/Characters/BadBean/Blueprints/BadBean_Anim_States Enum" :default "NewEnumerator0"))
  (message `/Game/Combat_Interface.Update_State` (`self.K2_GetPawn`) New_State))

(event `self.Update_BB_Bool`
  (params (BB_Key :type Name) (New_Value :type Boolean))
  (`BlackboardComponent.SetValueAsBool` (`AIBlueprintHelperLibrary.GetBlackboard` null) BB_Key New_Value))

(event `self.Set_Combat_Behavior`
  (params (New_Combat_Behavior :type "BehaviorTree Object Reference"))
  (bind _asbehavior_tree_component (cast `BehaviorTreeComponent` (`self.BrainComponent`)))
  (`BehaviorTreeComponent.SetDynamicSubtree` _asbehavior_tree_component (struct :`TagName` "Combat_Behavior") New_Combat_Behavior))

(fn `Do_Attack`
  (returns (Montage_Length :type "Float (double-precision)"))
  (bind _montage_length (message `/Game/Combat_Interface.Do_Attack` (`self.K2_GetPawn`)))
  (return _montage_length))

(fn `Get_Num_Patrol_Points`
  (returns (Num_Patrol_Points :type Integer))
  (bind _num_patrol_points (message `/Game/Combat_Interface.Get_Num_Patrol_Points` (`self.K2_GetPawn`)))
  (return _num_patrol_points))

(fn `Get_Patrol_Point`
  (params (Index :type Integer))
  (returns (Patrol_Point :type "Actor Object Reference"))
  (bind _patrol_point (message `/Game/Combat_Interface.Get_Patrol_Point` (`self.K2_GetPawn`) Index))
  (return _patrol_point))

(fn `Get_Target`
  (returns (Target :type "Actor Object Reference"))
  (bind _target (message `/Game/Combat_Interface.Get_Target` (`self.K2_GetPawn`)))
  (return _target))

(fn `UserConstructionScript`)
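; BP_Sword is a sword item that supplies the short-range melee combat behavior tree and drives its own animations.
; It forwards animation state changes and attack requests as messages to the Sword mesh's anim instance, returning the attack result to the caller.
; Patrol and target getters are stubs that report zero patrol points and no target.
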(event `self.ReceiveBeginPlay`
  (`parent.ReceiveBeginPlay`))

(event `/Game/BPI_Items.Set_Animation`
  (params (New_Anim_State :type Integer))
  (message `/Game/BPI_Items.Set_Animation` (`SkeletalMeshComponent.GetAnimInstance` (`self.Sword`)) New_Anim_State))

(fn `Do_Attack`
  (returns (Montage_Length :type "Float (double-precision)"))
  (bind _montage_length (message `/Game/Combat_Interface.Do_Attack` (`SkeletalMeshComponent.GetAnimInstance` (`self.Sword`))))
  (return _montage_length))

(fn `Get_Behavior`
  (returns (Behavior :type "BehaviorTree Object Reference"))
  (return "/Game/Characters/BadBean/Blueprints/AI/BT_Combat_ShortRangeMelee.BT_Combat_ShortRangeMelee"))

(fn `Get_Num_Patrol_Points`
  (returns (Num_Patrol_Points :type Integer))
  (return 0))

(fn `Get_Patrol_Point`
  (params (Index :type Integer))
  (returns (Patrol_Point :type "Actor Object Reference"))
  (return null))

(fn `Get_Target`
  (returns (Target :type "Actor Object Reference"))
  (return null))

(fn `UserConstructionScript`
  (`parent.UserConstructionScript`))
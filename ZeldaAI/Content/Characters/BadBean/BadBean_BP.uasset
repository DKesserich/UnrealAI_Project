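; BadBean_BP is an AI-controlled enemy character that patrols, holds a target and attacks with equipped items.
; On BeginPlay it spawns its default primary item, attaches it to a mesh socket and passes that item's behavior to the controller.
; An attack-range overlap toggles a blackboard bool for the target, and state changes reach the AnimInstance and both items.
; Attacks delegate to the primary item only when no secondary item exists.
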(event `self.ReceiveBeginPlay`
  (bind _default_primary_item (`self.Default_Primary_Item`))
  (if (`KismetSystemLibrary.IsValidClass` _default_primary_item)
    (bind _returnvalue (`|SpawnActorFromClass` _default_primary_item (`KismetMathLibrary.MakeTransform` (0.0 0.0 0.0)) "AlwaysSpawn" "MultiplyWithRoot" null null))
    (bind _output_get (set `self.Primary_Item` _returnvalue))
    (`self.K2_AttachToComponent` _output_get (`self.Mesh`) "Primary_Item" "SnapToTarget" "SnapToTarget" "KeepWorld" false)
    (bind _behavior (message `/Game/BPI_Items.Get_Behavior` _output_get))
    (message `/Game/Combat_Interface.Set_Combat_Behavior` (`self.GetController`) _behavior)))

(event `/Game/Combat_Interface.Update_State`
  (params (New_State :type "/Game/Characters/BadBean/Blueprints/BadBean_Anim_States Enum" :default "NewEnumerator0"))
  (bind _returnvalue (`KismetMathLibrary.Conv_ByteToInt` New_State))
  (message `/Game/Combat_Interface.Update_State` (`SkeletalMeshComponent.GetAnimInstance` (`self.Mesh`)) New_State)
  (message `/Game/BPI_Items.Set_Animation` (`self.Primary_Item`) _returnvalue)
  (message `/Game/BPI_Items.Set_Animation` (`self.Secondary_Item`) _returnvalue))

(event `/Game/Combat_Interface.Set_Target`
  (params (Target :type "Actor Object Reference"))
  (set `self.Target` Target))

(event `self.Attack_Range.OnComponentBeginOverlap`
  (params (OverlappedComponent :type "PrimitiveComponent Object Reference") (OtherActor :type "Actor Object Reference") (OtherComp :type "PrimitiveComponent Object Reference") (OtherBodyIndex :type Integer) (bFromSweep :type Boolean) (SweepResult :type "HitResult Structure (by ref)"))
  (if (== OtherActor (`self.Target`))
    (message `/Game/Combat_Interface.Update_BB_Bool` (`self.GetController`) "In_Attack_Range" true)))

(event `self.Attack_Range.OnComponentEndOverlap`
  (params (OverlappedComponent :type "PrimitiveComponent Object Reference") (OtherActor :type "Actor Object Reference") (OtherComp :type "PrimitiveComponent Object Reference") (OtherBodyIndex :type Integer))
  (if (== OtherActor (`self.Target`))
    (message `/Game/Combat_Interface.Update_BB_Bool` (`self.GetController`) "In_Attack_Range" false)))

(fn `Do_Attack`
  (returns (Montage_Length :type "Float (double-precision)"))
  (`/Engine/EditorBlueprintResources/StandardMacros.IsValid` (`self.Secondary_Item`)
    (:`Is Not Valid`
      (bind _montage_length (message `/Game/Combat_Interface.Do_Attack` (`self.Primary_Item`)))
      (return _montage_length))))

(fn `Get_Num_Patrol_Points`
  (returns (Num_Patrol_Points :type Integer))
  (return (`KismetArrayLibrary.Array_Length` (`self.Patrol_Points`))))

(fn `Get_Patrol_Point`
  (params (Index :type Integer))
  (returns (Patrol_Point :type "Actor Object Reference"))
  (return (`|GetArrayItem` (`self.Patrol_Points`) Index)))

(fn `Get_Target`
  (returns (Target :type "Actor Object Reference"))
  (return (`self.Target`)))

(fn `UserConstructionScript`)